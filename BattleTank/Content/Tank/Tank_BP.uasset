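; Player tank Blueprint that routes input to movement and aiming components and an orbiting camera.
; On BeginPlay it hands the left and right tracks to TankMovement and the barrel and turret to TankAiming.
; Forward and turn axes feed movement intents, and Fire calls the aiming component.
; Camera azimuth yaws a gimbal while elevation pitches the spring arm, keeping the two rotations separate.
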(event `self.ReceiveBeginPlay`
  (`TankMovementComponent.Initialize` (`self.TankMovement`) (`self.LeftTrack`) (`self.RightTrack`))
  (`TankAimingComponent.Initialize` (`self.TankAiming`) (`self.Barrel`) (`self.Turret`)))

(event `InputAction|Fire`
  (params (Key :type "Key Structure"))
  ;[1 1 1] Fire Control
  (:`Pressed`
    (`TankAimingComponent.Fire` (`self.TankAiming`))))

(event `InputAxis|TankForward`
  (params (AxisValue :type "Float (single-precision)"))
  ;[1 1 1] Go Forward and Backward
  (`TankMovementComponent.IntendMoveForward` (`self.TankMovement`) AxisValue))

(event `InputAxis|AimAzimuth`
  (params (AxisValue :type "Float (single-precision)"))
  ;[1 1 1] Camera Input Binding
  (`SceneComponent.K2_AddLocalRotation` (`self.Azimuth Gimbal`) (`KismetMathLibrary.MakeRotator` 0.0 0.0 AxisValue) false false))

(event `InputAxis|AimElevation`
  (params (AxisValue :type "Float (single-precision)"))
  ;[1 1 1] Camera Input Binding
  (`SceneComponent.K2_AddLocalRotation` (`self.SpringArm`) (`KismetMathLibrary.MakeRotator` 0.0 AxisValue) false false))

(event `InputAxis|TankRight`
  (params (AxisValue :type "Float (single-precision)"))
  ;[1 1 1] Turn Right and Left
  (`TankMovementComponent.IntendTurnRight` (`self.TankMovement`) AxisValue))

(fn `UserConstructionScript`)