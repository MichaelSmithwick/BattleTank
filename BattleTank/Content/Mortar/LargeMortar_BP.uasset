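; LargeMortar_BP is a large mortar that aims and fires through a TankAiming component.
; On BeginPlay it hands its barrel and turret to TankAiming and registers itself as MyTank on its HealthBar widget.
; Fire input calls TankAiming's Fire, while azimuth and elevation axes rotate the camera's gimbal yaw and spring arm pitch by the raw axis value.
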(event `self.ReceiveBeginPlay`
  (`TankAimingComponent.Initialize` (`self.TankAiming`) (`self.LargeMortarBarrel`) (`self.LargeMortarTurret`))
  (`self.InitialiseHealthBar`))

(event `InputAction|Fire`
  (params (Key :type "Key Structure"))
  ;[1 1 1] Fire Control
  (:`Pressed`
    (`TankAimingComponent.Fire` (`self.TankAiming`))))

(event `InputAxis|AimAzimuth`
  (params (AxisValue :type "Float (single-precision)"))
  ;[1 1 1] Camera Control
  (`SceneComponent.K2_AddLocalRotation` (`self.AzimuthGimbal`) (`KismetMathLibrary.MakeRotator` 0.0 0.0 AxisValue) false false))

(event `InputAxis|AimElevation`
  (params (AxisValue :type "Float (single-precision)"))
  ;[1 1 1] Camera Control
  (`SceneComponent.K2_AddLocalRotation` (`self.SpringArm`) (`KismetMathLibrary.MakeRotator` 0.0 AxisValue) false false))

(fn `InitialiseHealthBar`
  (bind _ashealth_bar (cast `/Game/UI/HealthBar` (`WidgetComponent.GetUserWidgetObject` (`self.Widget`))))
  (set `/Game/UI/HealthBar.MyTank` self _ashealth_bar))

(fn `UserConstructionScript`)